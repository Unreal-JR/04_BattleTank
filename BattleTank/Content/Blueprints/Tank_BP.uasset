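; Tank Blueprint that wires up its turret and barrel and handles orbit camera aiming input.
; BeginPlay passes the TankTurret and TankBarrel components to the turret and barrel reference setters.
; Azimuth input yaws the gimbal with a sensitivity multiplier, while elevation input pitches the spring arm, keeping the two rotation axes on separate components.
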(event EventBeginPlay
  (Class|Tank|SetTurretReference (Variables|Default|GetTankTurret))
  (Class|Tank|SetBarrelReference (Variables|Default|GetTankBarrel)))

(event Input|AxisEvents|InputAxisAimAximuth
  (params (AxisValue :type Float%20%28single-precision%29))
  ;[1 1 1] Camera Input Binding
  (Transformation|AddLocalRotation (Variables|Default|GetAximuth%20Gimble) (Math|Rotator|MakeRotator 0.0 0.0 (* AxisValue 1e+01)) false false))

(event Input|AxisEvents|InputAxisAimElevation
  (params (AxisValue :type Float%20%28single-precision%29))
  ;[1 1 1] Camera Input Binding
  (Transformation|AddLocalRotation (Variables|Default|GetSpringArm) (Math|Rotator|MakeRotator 0.0 AxisValue 0.0) false false))

(fn ConstructionScript)